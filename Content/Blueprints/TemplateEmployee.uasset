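; Template employee actor that joins the HUD's applicant list when the HUD's Recruit event fires.
; BeginPlay builds its info struct with a random portrait, creates a pickup prompt toggled by trigger overlap, and binds to Recruit.
; Recruiting removes the prompt, disables collision and refreshes applicants, without checking range.
; Initialize rolls skills and a skill-based salary; UseAction adds that salary to player money and destroys the actor.
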(event OnComponentBeginOverlap(Trigger)
  (params (OverlappedComponent :type Primitive%20Component%20Object%20Reference) (OtherActor :type Actor%20Object%20Reference) (OtherComp :type Primitive%20Component%20Object%20Reference) (OtherBodyIndex :type Integer) (bFromSweep :type Boolean) (SweepResult :type Hit%20Result%20Structure%20%28by%20ref%29))
  ;[1 1 1] Overlap Trigger Script
  (Utilities|Casting|CastToBP_Character OtherActor)
  (UserInterface|Viewport|AddtoViewport (Variables|Default|GetPickupTextReference) 0)
  (Variables|Default|SetisInRange? true))

(event OnComponentEndOverlap(Trigger)
  (params (OverlappedComponent :type Primitive%20Component%20Object%20Reference) (OtherActor :type Actor%20Object%20Reference) (OtherComp :type Primitive%20Component%20Object%20Reference) (OtherBodyIndex :type Integer))
  ;[1 1 1] Overlap Trigger Script
  (Utilities|Casting|CastToBP_Character OtherActor)
  (Widget|RemovefromParent (Variables|Default|GetPickupTextReference))
  (Variables|Default|SetisInRange? false))

(event Custom|PickupItem_Event_0
  (bind _characterreference (Variables|Default|GetCharacterReference))
  (bind _gamehudreference (Variables|/Game/Blueprints/BP_Character.BP_Character_C|GetGameHUDReference _characterreference))
  ;[1 1 1] Pick up and add items to the employee then refresh it.
  (Utilities|Array|Add (Variables|/Game/UI/GameHUD.GameHUD_C|GetApplicant _gamehudreference) (Variables|Default|GetItemInfo))
  (Widget|RemovefromParent (Variables|Default|GetPickupTextReference))
  (Rendering|SetActorHiddenInGame false)
  (Collision|SetActorEnableCollision false)
  (Default|RefreshApplicant _gamehudreference))

(event Custom|Initialize
  (bind _output_get (Variables|Default|SetEngineering (Math|Random|RandomIntegerinRange 0 (Variables|Default|GetEngineering%20Max))))
  (bind _output_get_2 (Variables|Default|SetMarketing (Math|Random|RandomIntegerinRange 0 (Variables|Default|GetMarketing%20Max))))
  (bind _output_get_3 (Variables|Default|SetManagement (Math|Random|RandomIntegerinRange 0 (Variables|Default|GetManagement%20Max))))
  (Variables|Default|SetSalary (Math|Random|RandomIntegerinRange (+ _output_get _output_get_2 _output_get_3) (* (+ _output_get _output_get_2 _output_get_3) 2))))

(event EventBeginPlay
  (bind _employeeimages (Variables|Default|GetEmployeeImages))
  ;[1 1 1] Event Begin Play
  (Variables|Default|SetItemInfo (Utilities|Struct|MakeEmployeeStructure 0 (Utilities|Array|Get(acopy) _employeeimages (Math|Random|RandomInteger (Utilities|Array|Length _employeeimages))) "EmployeeA" "EmployeeA Action"))
  (bind _returnvalue (UserInterface|CreateWidget "/Game/UI/PickupText.PickupText_C"))
  (Variables|Default|SetPickupTextReference _returnvalue)
  (Utilities|Struct|SetmembersinEmployeeStructure (Variables|Default|GetItemInfo) self)
  (Variables|/Game/UI/PickupText.PickupText_C|SetPickupActor (Variables|Default|GetPickupTextReference) (.Employee (Utilities|Struct|BreakEmployeeStructure (Variables|Default|GetItemInfo))))
  (Variables|/Game/UI/PickupText.PickupText_C|SetPickupText (Variables|Default|GetPickupTextReference) (.PickupText (Utilities|Struct|BreakEmployeeStructure (Variables|Default|GetItemInfo))))
  (bind _asbp_character (Utilities|Casting|CastToBP_Character (Game|GetPlayerCharacter 0)))
  (bind _output_get (Variables|Default|SetCharacterReference _asbp_character))
  (bind _asgame_hud (Utilities|Casting|CastToGameHUD (Variables|/Game/Blueprints/BP_Character.BP_Character_C|GetGameHUDReference _asbp_character)))
  (EventDispatchers|BindEventtoRecruit _asgame_hud (delegate Custom|PickupItem_Event_0)))

(event EventUseAction
  (bind _characterreference (Variables|Default|GetCharacterReference))
  ;[1 1 1] Use Action
  (Variables|/Game/Blueprints/BP_Character.BP_Character_C|SetMoney _characterreference (+ (Variables|/Game/Blueprints/BP_Character.BP_Character_C|GetMoney _characterreference) (Variables|Default|GetSalary)))
  (Actor|DestroyActor))

(fn ConstructionScript)