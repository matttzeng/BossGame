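; TemplateQuest is a quest Blueprint that runs a timed wheat transaction on the player's BP_Character.
; StartQuest deducts PriceDown from the character's AmountOfWheat, then waits QuestDuration with a Delay.
; It then adds the same PriceDown back, clears QuestActive and passes QuestHUB to the character's RemoveQuest.
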(event Custom|StartQuest
  (bind _pricedown (Variables|Default|GetPriceDown))
  (bind _asbp_character (Utilities|Casting|CastToBP_Character (Game|GetPlayerCharacter 0)))
  (Variables|/Game/Blueprints/BP_Character.BP_Character_C|SetAmountOfWheat _asbp_character (- (Variables|/Game/Blueprints/BP_Character.BP_Character_C|GetAmountOfWheat _asbp_character) _pricedown))
  (Utilities|FlowControl|Delay (Variables|Default|GetQuestDuration))
  (Variables|/Game/Blueprints/BP_Character.BP_Character_C|SetAmountOfWheat _asbp_character (+ (Variables|/Game/Blueprints/BP_Character.BP_Character_C|GetAmountOfWheat _asbp_character) _pricedown))
  (Variables|Default|SetQuestActive? false)
  (Default|RemoveQuest _asbp_character (Variables|Default|GetQuestHUB)))

(event EventBeginPlay)

(event Collision|EventActorBeginOverlap
  (params (OtherActor :type Actor%20Object%20Reference)))

(event EventTick
  (params (DeltaSeconds :type Float%20%28single-precision%29)))

(fn ConstructionScript)