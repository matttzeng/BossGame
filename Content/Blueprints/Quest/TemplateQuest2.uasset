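; TemplateQuest2 is a timed quest Blueprint that temporarily takes wheat from the player character.
; StartQuest subtracts its price from BP_Character's wheat count, waits for the quest duration, then adds the same amount back.
; It then clears its active flag and has the character remove the quest via QuestHUB.
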(event Custom|StartQuest
  (bind _pricedown_0 (Variables|Default|GetPriceDown_0))
  (bind _asbp_character (Utilities|Casting|CastToBP_Character (Game|GetPlayerCharacter 0)))
  (Variables|/Game/Blueprints/BP_Character.BP_Character_C|SetAmountOfWheat _asbp_character (- (Variables|/Game/Blueprints/BP_Character.BP_Character_C|GetAmountOfWheat _asbp_character) _pricedown_0))
  (Utilities|FlowControl|Delay (Variables|Default|GetQuestDuration_0))
  (Variables|/Game/Blueprints/BP_Character.BP_Character_C|SetAmountOfWheat _asbp_character (+ (Variables|/Game/Blueprints/BP_Character.BP_Character_C|GetAmountOfWheat _asbp_character) _pricedown_0))
  (Variables|Default|SetQuestActive? false)
  (Default|RemoveQuest _asbp_character (Variables|Default|GetQuestHUB)))

(event EventBeginPlay)

(event Collision|EventActorBeginOverlap
  (params (OtherActor :type Actor%20Object%20Reference)))

(event EventTick
  (params (DeltaSeconds :type Float%20%28single-precision%29)))

(fn ConstructionScript)