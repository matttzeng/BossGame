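; CB_GameModeBase is a game mode Blueprint that handles spending money on objects.
; CanAffordObject casts to CB_GameState and checks whether CurrentMoney covers a given amount.
; ObjectBought repeats that check and, when it passes, subtracts the amount from CurrentMoney in the game state.
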(event EventBeginPlay)

(event EventTick
  (params (DeltaSeconds :type Float%20%28single-precision%29)))

(fn ConstructionScript)

(fn CanAffordObject
  (params (ObjectAmount :type Integer))
  (bind _ascb_game_state (Utilities|Casting|CastToCB_GameState (Game|GetGameState)))
  (return (>= (Variables|/Game/Blueprints/CB_GameState.CB_GameState_C|GetCurrentMoney _ascb_game_state) ObjectAmount)))

(fn ObjectBought
  (params (ObjectAmount :type Integer))
  (bind _canafford (CallFunction|CanAffordObject ObjectAmount))
  (if _canafford
    (bind _ascb_game_state (Utilities|Casting|CastToCB_GameState (Game|GetGameState)))
    (Variables|/Game/Blueprints/CB_GameState.CB_GameState_C|SetCurrentMoney _ascb_game_state (- (Variables|/Game/Blueprints/CB_GameState.CB_GameState_C|GetCurrentMoney _ascb_game_state) ObjectAmount))))