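; PC_MouseControl creates the game HUD widget and adds it to the viewport on BeginPlay.
; An unconnected FlipFlop, which never runs, holds an inventory UI toggle that casts the HUD to UI and shows or hides a button and text blocks.
; That toggle ignores look input while open and resets it when closed, but leaves the mouse cursor shown in both states.
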(event EventBeginPlay
  (bind _returnvalue (UserInterface|CreateWidget "/Game/UI/GameHUD.GameHUD_C"))
  (UserInterface|Viewport|AddtoViewport _returnvalue 0))

(event Input|KeyboardEvents|T
  (params (Key :type Key%20Structure :default "None"))
  ;[1 1 1] Open Inventory UI, lock look input
)

(fn ConstructionScript)