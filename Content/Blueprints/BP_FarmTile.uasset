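; Farm tile actor where the player plants wheat, corn or pumpkin seeds and harvests the grown crop.
; PlatSeed spends the character's selected seed, then GrowTime macros count down on a Text3D while mesh components are swapped per stage.
; ChanceOfDisease rolls at each stage, halting growth with a diseased material on failure.
; Activate calls Harvest, which clears finished or diseased plants and spawns loose produce only for healthy ones.
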(event Custom|PlantPumpkin
  (bind _relative_transformlocation (Variables|Default|GetRelative%20TransformLocation))
  (bind _returnvalue (AddComponent|AddStaticMeshComponent false (Math|Transform|MakeTransform _relative_transformlocation "0, 0, 0" "1,1,1")))
  (Utilities|GrowTime (Variables|Default|GetPumpkinGrowTime)
    (:Out
      (Utilities|ChanceOfDisease _returnvalue
        (:NoDisease
          (Components|DestroyComponent _returnvalue)
          (bind _returnvalue_2 (AddComponent|AddStaticMeshComponent false (Math|Transform|MakeTransform _relative_transformlocation "0, 0, 0" "1,1,1")))
          (Utilities|GrowTime (Variables|Default|GetPumpkinGrowTime)
            (:Out
              (Utilities|ChanceOfDisease _returnvalue_2
                (:NoDisease
                  (Components|DestroyComponent _returnvalue_2)
                  (bind _returnvalue_3 (AddComponent|AddStaticMeshComponent false (Math|Transform|MakeTransform _relative_transformlocation "0, 0, 0" "1,1,1")))
                  (Utilities|ChanceOfDisease _returnvalue_3
                    (:NoDisease
                      (Variables|Default|SetFullyGrown? true)
                      (Variables|Default|SetCurrentMesh _returnvalue_3)
                      (Variables|Default|SetWhatCanBeHarvested "Pumpkin"))))))))))))

(event Custom|PlantWheat
  (bind _relative_transformlocation (Variables|Default|GetRelative%20TransformLocation))
  (bind _returnvalue (AddComponent|AddStaticMeshComponent false (Math|Transform|MakeTransform _relative_transformlocation "0, 0, 0" "1,1,1")))
  (Utilities|GrowTime (Variables|Default|GetWheatGrowTime)
    (:Out
      (Utilities|ChanceOfDisease _returnvalue
        (:NoDisease
          (Components|DestroyComponent _returnvalue)
          (bind _returnvalue_2 (AddComponent|AddStaticMeshComponent false (Math|Transform|MakeTransform _relative_transformlocation "0, 0, 0" "1,1,1")))
          (Utilities|GrowTime (Variables|Default|GetWheatGrowTime)
            (:Out
              (Utilities|ChanceOfDisease _returnvalue_2
                (:NoDisease
                  (Components|DestroyComponent _returnvalue_2)
                  (bind _returnvalue_3 (AddComponent|AddStaticMeshComponent false (Math|Transform|MakeTransform _relative_transformlocation "0, 0, 0" "1,1,1")))
                  (Utilities|ChanceOfDisease _returnvalue_3
                    (:NoDisease
                      (Variables|Default|SetFullyGrown? true)
                      (Variables|Default|SetCurrentMesh _returnvalue_3)
                      (Variables|Default|SetWhatCanBeHarvested "Wheat"))))))))))))

(event Custom|PlantCorn
  (bind _relative_transformlocation (Variables|Default|GetRelative%20TransformLocation))
  (bind _returnvalue (AddComponent|AddStaticMeshComponent false (Math|Transform|MakeTransform _relative_transformlocation "0, 0, 0" "1,1,1")))
  (Utilities|GrowTime (Variables|Default|GetCornGrowTime)
    (:Out
      (Utilities|ChanceOfDisease _returnvalue
        (:NoDisease
          (Components|DestroyComponent _returnvalue)
          (bind _returnvalue_2 (AddComponent|AddStaticMeshComponent false (Math|Transform|MakeTransform _relative_transformlocation "0, 0, 0" "1,1,1")))
          (Utilities|GrowTime (Variables|Default|GetCornGrowTime)
            (:Out
              (Utilities|ChanceOfDisease _returnvalue_2
                (:NoDisease
                  (Components|DestroyComponent _returnvalue_2)
                  (bind _returnvalue_3 (AddComponent|AddStaticMeshComponent false (Math|Transform|MakeTransform _relative_transformlocation "0, 0, 0" "1,1,1")))
                  (Utilities|ChanceOfDisease _returnvalue_3
                    (:NoDisease
                      (Variables|Default|SetFullyGrown? true)
                      (Variables|Default|SetCurrentMesh _returnvalue_3)
                      (Variables|Default|SetWhatCanBeHarvested "Corn"))))))))))))

(event EventActivate
  (CallFunction|Harvest))

(event EventPlatSeed
  (if (not (Variables|Default|GetIsSomethingPlanted?))
    (bind _asthird_person_character (Utilities|Casting|CastToThirdPersonCharacter (Game|GetPlayerCharacter 0)))
    (switch int (Variables|/Game/ThirdPersonBP/Blueprints/ThirdPersonCharacter.ThirdPersonCharacter_C|GetSeed _asthird_person_character)
      (:0
        (Utilities|DoWeHaveWheatSeed
          (:Out
            (CallFunction|PlantWheat))))
      (:1
        (Utilities|DoWeHaveCornSeed
          (:Out
            (CallFunction|PlantCorn))))
      (:2
        (Utilities|DoWeHavePumpkinSeed
          (:Out
            (CallFunction|PlantPumpkin)))))
    (Variables|Default|SetIsSomethingPlanted? true)))

(event EventBeginPlay
  (Class|Text3DComponent|SetText (Variables|Default|GetText3D) (Variables|Default|GetValue)))

(fn ConstructionScript)

(fn Harvest
  (bind _text3d (Variables|Default|GetText3D))
  (bind _returnvalue (Transformation|GetWorldLocation _text3d))
  (bind _returnvalue_2 (Math|Conversions|ToTransform(Vector) _returnvalue))
  (if (Variables|Default|GetFullyGrown?)
    (Components|DestroyComponent (Variables|Default|GetCurrentMesh))
    (switch string (Variables|Default|GetWhatCanBeHarvested)
      (:Default
        _)
      (:Wheat
        (Game|SpawnActorfromClass "/Game/Blueprints/BP_WheatLoose.BP_WheatLoose_C" _returnvalue_2 "Undefined" 0 0))
      (:Corn
        (Game|SpawnActorfromClass "/Game/Blueprints/BP_CornLoose.BP_CornLoose_C" _returnvalue_2 "Undefined" 0 0))
      (:Pumpkin
        (Game|SpawnActorfromClass "/Game/Blueprints/BP_PumpkinLoose.BP_PumpkinLoose_C" _returnvalue_2 "Undefined" 0 0)))
    (Variables|Default|SetFullyGrown? false)
    (Variables|Default|SetCurrentMesh 0)
    (Variables|Default|SetIsSomethingPlanted? false)
    (Variables|Default|SetWhatCanBeHarvested "")))