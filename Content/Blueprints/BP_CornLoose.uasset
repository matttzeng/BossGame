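; BP_CornLoose is a loose corn pickup actor that the player character collects by touching it.
; When its Box component overlaps a BP_Character, it increments that character's AmountOfCorn and destroys itself.
; An unconnected leftover chain would grant corn to player 0 after a delay, but it never runs.
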(event OnComponentBeginOverlap(Box)
  (params (OverlappedComponent :type Primitive%20Component%20Object%20Reference) (OtherActor :type Actor%20Object%20Reference) (OtherComp :type Primitive%20Component%20Object%20Reference) (OtherBodyIndex :type Integer) (bFromSweep :type Boolean) (SweepResult :type Hit%20Result%20Structure%20%28by%20ref%29))
  (bind _asbp_character (Utilities|Casting|CastToBP_Character OtherActor))
  (bind _result (Math|Integer|IncrementInt (Variables|/Game/Blueprints/BP_Character.BP_Character_C|GetAmountOfCorn _asbp_character))
    (:%20%20
      (Variables|/Game/Blueprints/BP_Character.BP_Character_C|SetAmountOfCorn _asbp_character _result)
      (Actor|DestroyActor))))

(event EventBeginPlay)

(event Collision|EventActorBeginOverlap
  (params (OtherActor :type Actor%20Object%20Reference)))

(event EventTick
  (params (DeltaSeconds :type Float%20%28single-precision%29)))

(fn ConstructionScript)